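; Player-driven tank Blueprint that wires input to its aiming, movement and track components.
; On BeginPlay it hands the barrel and turret to TankAiming and both tracks to TankMovement.
; Aim axes rotate the Gimbal (yaw) and SpringArm (pitch), and Fire calls TankAiming.Fire.
; Driving works either through per-track throttle and decelerate axes or through forward and turn intents sent to TankMovement.
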(event EventBeginPlay
  (Class|TankAimingComponent|Initialize (Variables|Default|GetTankAiming) (Variables|Default|GetTankBarrel) (Variables|Default|GetTankTurret))
  (Class|TankMovementComponent|Initialize (Variables|Default|GetTankMovement) (Variables|Default|GetLeft%20Track) (Variables|Default|GetRight%20Track)))

(event Input|ActionEvents|InputActionFire
  (params (Key :type Key%20Structure))
  ;[1 1 1] Tank Input
  (:Pressed
    (Class|TankAimingComponent|Fire (Variables|Default|GetTankAiming))))

(event Input|AxisEvents|InputAxisAimTurret
  (params (AxisValue :type Float%20%28single-precision%29))
  ;[1 1 1] Tank Input
  (Transformation|AddLocalRotation (Variables|Default|GetGimbal) (Math|Rotator|MakeRotator 0.0 0.0 AxisValue) false false))

(event Input|AxisEvents|InputAxisAimBarrel
  (params (AxisValue :type Float%20%28single-precision%29))
  ;[1 1 1] Tank Input
  (Transformation|AddLocalRotation (Variables|Default|GetSpringArm) (Math|Rotator|MakeRotator 0.0 AxisValue 0.0) false false))

(event Input|AxisEvents|InputAxisLeftTrackThrottle
  (params (AxisValue :type Float%20%28single-precision%29))
  ;[1 1 1] Tank Movement
  (Class|TankTrack|SetThrottle (Variables|Default|GetLeft%20Track) AxisValue))

(event Input|AxisEvents|InputAxisRightTrackThrottle
  (params (AxisValue :type Float%20%28single-precision%29))
  ;[1 1 1] Tank Movement
  (Class|TankTrack|SetThrottle (Variables|Default|GetRight%20Track) AxisValue))

(event Input|AxisEvents|InputAxisLeftTrackDecelerate
  (params (AxisValue :type Float%20%28single-precision%29))
  ;[1 1 1] Tank Movement
  (Class|TankTrack|SetThrottle (Variables|Default|GetLeft%20Track) AxisValue))

(event Input|AxisEvents|InputAxisMoveForward
  (params (AxisValue :type Float%20%28single-precision%29))
  ;[1 1 1] Tank Input
  (Class|TankMovementComponent|IntendMoveForward (Variables|Default|GetTankMovement) AxisValue))

(event Input|AxisEvents|InputAxisRightTrackDecelerate
  (params (AxisValue :type Float%20%28single-precision%29))
  ;[1 1 1] Tank Movement
  (Class|TankTrack|SetThrottle (Variables|Default|GetRight%20Track) AxisValue))

(event Input|AxisEvents|InputAxisTurnRight
  (params (AxisValue :type Float%20%28single-precision%29))
  ;[1 1 1] Tank Input
  (Class|TankMovementComponent|IntendMoveRight (Variables|Default|GetTankMovement) AxisValue))

(fn ConstructionScript)